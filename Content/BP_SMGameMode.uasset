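; BP_SMGameMode is the game mode that runs the start menu and handles the switch into the House level.
; On BeginPlay it creates and stores the BP_UIStartMenu widget, adds it to the viewport and shows the mouse cursor.
; LoadHouseLevel brings in House as a level instance rather than opening a new map, then hides the menu and cursor and switches input to game only.
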(event `self.ReceiveBeginPlay`
  (bind _returnvalue (`|CreateWidget` "/Game/UI/BP_UIStartMenu.BP_UIStartMenu_C"))
  (bind _output_get (set `self.StartMenu` _returnvalue))
  (`UserWidget.AddToViewport` _output_get 0)
  (set `PlayerController.bShowMouseCursor` true (`GameplayStatics.GetPlayerController` 0)))

(fn `LoadHouseLevel`
  (bind _returnvalue (`GameplayStatics.GetPlayerController` 0))
  (`LevelStreamingDynamic.LoadLevelInstance` "House" (0.0 0.0 0.0) (struct) "" null)
  (`Widget.SetVisibility` (`self.StartMenu`) "Hidden")
  (set `PlayerController.bShowMouseCursor` false _returnvalue)
  (`WidgetBlueprintLibrary.SetInputMode_GameOnly` _returnvalue))

(fn `UserConstructionScript`)