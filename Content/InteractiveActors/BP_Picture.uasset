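; BP_Picture is an interactive picture actor that launches an image puzzle, available once the game mode's TalkWithHana flag is set.
; Entering its sphere shows the SelectObject marker and registers the actor with BP_GameMode as the in-range interactive object.
; Leaving only hides the marker, without clearing the game mode's references.
; Interact calls LoadImagePuzzle on the game mode and disables the sphere's collision.
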(event `self.ReceiveBeginPlay`
  (bind _asbp_game_mode (cast `/Game/BP_GameMode` (`GameplayStatics.GetGameMode`)))
  (set `self.As BP Game Mode` _asbp_game_mode))

(event `self.Sphere.OnComponentBeginOverlap`
  (params (OverlappedComponent :type "PrimitiveComponent Object Reference") (OtherActor :type "Actor Object Reference") (OtherComp :type "PrimitiveComponent Object Reference") (OtherBodyIndex :type Integer) (bFromSweep :type Boolean) (SweepResult :type "HitResult Structure (by ref)"))
  (bind _as_bp_game_mode (`self.As BP Game Mode`))
  (bind _selectobject (`self.SelectObject`))
  (if (`/Game/BP_GameMode.TalkWithHana` (`self.As BP Game Mode`))
    (`SceneComponent.SetVisibility` _selectobject true false)
    (set `/Game/BP_GameMode.InArea` (`SceneComponent.bVisible` _selectobject) _as_bp_game_mode)
    (set `/Game/BP_GameMode.InteractiveObject` self _as_bp_game_mode)))

(event `self.Sphere.OnComponentEndOverlap`
  (params (OverlappedComponent :type "PrimitiveComponent Object Reference") (OtherActor :type "Actor Object Reference") (OtherComp :type "PrimitiveComponent Object Reference") (OtherBodyIndex :type Integer))
  (`SceneComponent.SetVisibility` (`self.SelectObject`) false false))

(event `/Game/BP_Interface.Interact`
  (`/Game/BP_GameMode.LoadImagePuzzle` (`self.As BP Game Mode`))
  (`PrimitiveComponent.SetCollisionEnabled` (`self.Sphere`) "NoCollision"))

(fn `UserConstructionScript`)