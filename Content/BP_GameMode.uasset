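; Game mode that owns the pause menu and gameplay UI widgets and exposes functions to show them.
; BeginPlay creates both widgets; Pause toggles the menu's visibility, the mouse cursor and the game's paused state together.
; LoadImagePuzzle shows the puzzle panel with UI-only input and a cursor, while LoadDialogue shows the dialogue panel and sets an in-dialogue flag.
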(event `self.ReceiveBeginPlay`
  (`|ExecutionSequence`
    (:`then_0`
      (bind _returnvalue (`|CreateWidget` "/Game/BP_UIPause.BP_UIPause_C"))
      (set `self.PauseMenu` _returnvalue))
    (:`then_1`
      (bind _returnvalue_2 (`|CreateWidget` "/Game/BP_UIGameplay.BP_UIGameplay_C"))
      (set `self.UIGameplay` _returnvalue_2))))

(event `self.ReceiveTick`
  (params (DeltaSeconds :type "Float (single-precision)")))

(fn `LoadDialogue`
  (bind _uigameplay (`self.UIGameplay`))
  (`Widget.SetVisibility` (`/Game/BP_UIGameplay.Dialogue` _uigameplay) "Visible")
  (`UserWidget.AddToViewport` _uigameplay 0)
  (set `self.IsInDialogue` true))

(fn `LoadImagePuzzle`
  (bind _returnvalue (`GameplayStatics.GetPlayerController` 0))
  (bind _uigameplay (`self.UIGameplay`))
  (`Widget.SetVisibility` (`/Game/BP_UIGameplay.ImagePuzzle` _uigameplay) "Visible")
  (`UserWidget.AddToViewport` _uigameplay 0)
  (`WidgetBlueprintLibrary.SetInputMode_UIOnlyEx` _returnvalue _uigameplay)
  (set `PlayerController.bShowMouseCursor` true _returnvalue))

(fn `Pause`
  (params (isPaused :type Boolean))
  (bind _pausemenu (`self.PauseMenu`))
  (`Widget.SetVisibility` _pausemenu (select `bool` isPaused :`false` "Hidden" :`true` "Visible" :!type "ESlateVisibility Enum"))
  (`UserWidget.AddToViewport` _pausemenu 0)
  (set `PlayerController.bShowMouseCursor` isPaused (`GameplayStatics.GetPlayerController` 0))
  (`GameplayStatics.SetGamePaused` isPaused))

(fn `UserConstructionScript`)